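; Health potion item Blueprint that restores player health when used.
; Its UseItem override calls the parent, finds the 2DSideScrollerCharacter with GetActorOfClass, and adds AmountToRestore to that character's CurrentHealth.
; The result is clamped to MaxHealth and the function always returns true.
; The event graph and construction script add no behavior of their own.
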(fn `UseItem`
  (returns (Success :type Boolean))
  (`parent.UseItem`)
  (bind _returnvalue (`GameplayStatics.GetActorOfClass` "/Game/2DSideScrollerBP/Blueprints/2DSideScrollerCharacter.2DSideScrollerCharacter_C"))
  (bind _output_get (set `MainCharacter.CurrentHealth` (+ (`MainCharacter.CurrentHealth` _returnvalue) (`self.AmountToRestore`)) _returnvalue))
  (bind _maxhealth (`MainCharacter.MaxHealth` _returnvalue))
  (if (> _output_get _maxhealth)
    (set `MainCharacter.CurrentHealth` _maxhealth _returnvalue))
  (return true))

(fn `UserConstructionScript`
  (`parent.UserConstructionScript`))