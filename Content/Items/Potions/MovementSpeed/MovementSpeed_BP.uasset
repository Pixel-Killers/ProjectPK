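; Movement speed potion item that temporarily boosts the side-scroller player character's walk speed.
; Its UseItem override calls the parent, finds the 2DSideScrollerCharacter with GetActorOfClass, and multiplies its MaxWalkSpeed by AmountToScale.
; It then sets a ten-second timer by function name that calls ResetMovementSpeed on the character to undo the boost, and returns true.
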(fn `UseItem`
  (returns (Success :type Boolean))
  (`parent.UseItem`)
  (bind _returnvalue (`GameplayStatics.GetActorOfClass` "/Game/2DSideScrollerBP/Blueprints/2DSideScrollerCharacter.2DSideScrollerCharacter_C"))
  (bind _charactermovement (`Character.CharacterMovement` _returnvalue))
  (set `CharacterMovementComponent.MaxWalkSpeed` (* (`CharacterMovementComponent.MaxWalkSpeed` _charactermovement) (`self.AmountToScale`)) _charactermovement)
  (`KismetSystemLibrary.K2_SetTimer` _returnvalue "ResetMovementSpeed" 10.0)
  (return true))

(fn `UserConstructionScript`
  (`parent.UserConstructionScript`))