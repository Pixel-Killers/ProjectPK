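; Basic 2D side-scroller ground enemy that patrols a fixed stretch beside its spawn, chases the player on sight and shoots when close.
; Tick drives patrol, chase, flipbook switching and a delayed target drop that applies outside attack range.
; AttackRange overlaps start and clear a looping timer that fires BulletBP projectiles aimed at the target.
; NotifyDamage briefly tints the sprite red, while TakeDamage reduces health and destroys the enemy at zero.
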(event `self.ReceiveBeginPlay`
  (set `self.InitLocation` (`self.K2_GetActorLocation`))
  (set `self.OriginalColor` (`PaperFlipbookComponent.SpriteColor` (`self.Sprite`))))

(event `self.ReceiveTick`
  (params (DeltaSeconds :type "Float (single-precision)"))
  (bind _target (`self.Target`))
  (`self.Stop Following`)
  (`self.Patrol`)
  (if (`self.IsAttackAnim`)
    (`PaperFlipbookComponent.SetFlipbook` (`self.Sprite`) "/Game/Enemies/BasicEnemy/Animations/Attack/GroundEnemy_Attack.GroundEnemy_Attack")
    (`KismetSystemLibrary.Delay` 0.14)
    (set `self.IsAttackAnim` false))
  (`self.UpdateAnimation` "/Game/Enemies/BasicEnemy/Animations/Idle/GroundEnemy_Idle.GroundEnemy_Idle" "/Game/Enemies/BasicEnemy/Animations/Run/GroundEnemy_Run.GroundEnemy_Run")
  (`/Engine/EditorBlueprintResources/StandardMacros.IsValid` _target
    (:`Is Valid`
      (`self.Move Towards Player` _target))))

(event `self.Front Sight.OnSeePawn`
  (params (Pawn :type "Pawn Object Reference"))
  ;[1 1 1] Zaidejas yra vejamasis, kai yra pamatomas
  (`self.Move Towards Player` Pawn "/Game/Enemies/BasicEnemy/Animations/Run/GroundEnemy_Run.GroundEnemy_Run"))

(event `Stop Following`
  ;[1 1 1] ZIurima kada nustoti vytis
  (`/Engine/EditorBlueprintResources/StandardMacros.IsValid` (`self.Target`)
    (:`Is Valid`
      (bind _istargetless (`self.Compare X Coords`))
      (`self.Update Rotation` _istargetless)
      (`KismetSystemLibrary.Delay` 3.0)
      (if (not (`self.ShouldAttack`))
        (set `self.Target` null)))
    (:`Is Not Valid`
      (`NavMovementComponent.StopActiveMovement` (`self.CharacterMovement`)))))

(event `self.Attack Range.OnComponentBeginOverlap`
  (params (OverlappedComponent :type "PrimitiveComponent Object Reference") (OtherActor :type "Actor Object Reference") (OtherComp :type "PrimitiveComponent Object Reference") (OtherBodyIndex :type Integer) (bFromSweep :type Boolean) (SweepResult :type "HitResult Structure (by ref)"))
  (`self.Begin Attack` OtherActor (delegate `Attack`)))

(event `NotifyDamage`
  ;[1 1 1] Parodo, kad patyre zala
  (`PaperFlipbookComponent.SetSpriteColor` (`self.Sprite`) (struct :`R` 0.642361 :`A` 1.0))
  (`KismetSystemLibrary.Delay` 0.3)
  (`PaperFlipbookComponent.SetSpriteColor` (`self.Sprite`) (`self.OriginalColor`)))

(event `self.Attack Range.OnComponentEndOverlap`
  (params (OverlappedComponent :type "PrimitiveComponent Object Reference") (OtherActor :type "Actor Object Reference") (OtherComp :type "PrimitiveComponent Object Reference") (OtherBodyIndex :type Integer))
  (`self.End Attack` OtherActor (delegate `Attack`)))

(event `Attack`
  (bind _location (.location (`SceneComponent.K2_GetComponentToWorld` (`self.BulletSpawn`))))
  ;[1 1 1] Atakos logika. Reikia tvarkymo su animacijom ir laikais!
  (`|ExecutionSequence`
    (:`then_0`
      (set `self.IsAttackAnim` true))
    (:`then_1`
      (bind _returnvalue (`|SpawnActorFromClass` "/Game/Enemies/RangedAttack/Animations/Bullet/BulletBP.BulletBP_C" (`KismetMathLibrary.MakeTransform` _location (`KismetMathLibrary.FindLookAtRotation` _location (`self.K2_GetActorLocation` (`self.Target`))) (.scale (`SceneComponent.K2_GetComponentToWorld` (`self.BulletSpawn`)))) "Undefined" "OverrideRootScale" null null))
      (set `/Game/Enemies/RangedAttack/Animations/RangedAttack.BaseDamage` 10 _returnvalue))))

(fn `Begin Attack`
  (params (Object :type "Object Object Reference") (Delegate :type Delegate))
  (bind _as2dside_scroller_character (cast `/Game/2DSideScrollerBP/Blueprints/2DSideScrollerCharacter` Object))
  (set `self.Target` _as2dside_scroller_character)
  (set `self.ShouldAttack` true)
  (`KismetSystemLibrary.K2_SetTimerDelegate` Delegate 2.0 true)
  (`NavMovementComponent.StopActiveMovement` (`self.CharacterMovement`))
  (return))

(fn `Compare X Coords`
  (returns (IsTargetLess :type Boolean))
  (return (< (.x (`self.K2_GetActorLocation` (`self.Target`))) (.x (`self.K2_GetActorLocation`)))))

(fn `Die`
  (`self.K2_DestroyActor`))

(fn `End Attack`
  (params (Object :type "Object Object Reference") (Delegate :type Delegate))
  (cast `/Game/2DSideScrollerBP/Blueprints/2DSideScrollerCharacter` Object)
  (set `self.ShouldAttack` false)
  (`KismetSystemLibrary.K2_SetTimerDelegate` Delegate)
  (return))

(fn `Move Towards Player`
  (params (Player :type "Object Object Reference") (Begimas :type "PaperFlipbook Object Reference"))
  (bind _as2dside_scroller_character (cast `/Game/2DSideScrollerBP/Blueprints/2DSideScrollerCharacter` Player)
    (:`then`
      (if (not (`self.ShouldAttack`))
        (`AIBlueprintHelperLibrary.SimpleMoveToActor` (`AIBlueprintHelperLibrary.GetAIController` self) _as2dside_scroller_character)
        ;[1 1 1 1 11] Darom tik cia, kad neglitchintu animacija
        (`/Engine/EditorBlueprintResources/StandardMacros.IsValid` (`self.Target`)
          (:`Is Valid`
            _)
          (:`Is Not Valid`
            (`PaperFlipbookComponent.SetFlipbook` (`self.Sprite`) Begimas)
            (set `self.Target` _as2dside_scroller_character)))))
    (:`CastFailed`
      _))
  (return))

(fn `Patrol`
  (bind _x (.x (- (`self.K2_GetActorLocation`) (`self.InitLocation`))))
  ;[1 1 1 1 12] Vykdom, kai nereikia pulti
  (if (not (`self.ShouldAttack`))
    ;[1 1 1 1 12] Vykdom tik, kai nesivejamas zaidejas
    (`/Engine/EditorBlueprintResources/StandardMacros.IsValid` (`self.Target`)
      (:`Is Valid`
        _)
      (:`Is Not Valid`
        (`self.K2_SetActorRotation` (`KismetMathLibrary.SelectRotator` (struct) (struct :`Yaw` 180.0) (`self.MovingRight`)))
        (`self.AddMovementInput` (`KismetMathLibrary.SelectVector` (1.0 0.0 0.0) (-1.0 0.0 0.0) (`self.MovingRight`)) (* (`GameplayStatics.GetWorldDeltaSeconds`) (`self.MovementSpeed`)))
        (if (<= _x -1200.0)
          (set `self.MovingRight` true)
          (elif (>= _x 0.0)
            (set `self.MovingRight` false))))))
  (return))

(fn `TakeDamage`
  (params (Damage :type Integer))
  (bind _output_get (set `self.Health` (- (`self.Health`) Damage)))
  (if (<= _output_get 0)
    (`self.K2_DestroyActor`)))

(fn `Update Rotation`
  (params (`Is Target X Less` :type Boolean))
  (if `Is Target X Less`
    (`self.K2_SetActorRotation` (struct :`Yaw` 180.0))
    (else
      (`self.K2_SetActorRotation` (struct))))
  (return))

(fn `UpdateAnimation`
  (params (Stovejimas :type "PaperFlipbook Object Reference") (Ejimas :type "PaperFlipbook Object Reference"))
  (`PaperFlipbookComponent.SetFlipbook` (`self.Sprite`) (select `bool` (> (`KismetMathLibrary.VSize` (`self.GetVelocity`)) 0.0) :`false` Stovejimas :`true` Ejimas))
  (return))

(fn `UserConstructionScript`)