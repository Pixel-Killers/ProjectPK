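; Flying bat melee enemy for a 2D side-scroller, using inherited construction logic and flipbook animation.
; A looping timer triggers attacks while IsAttacking is set, damaging the target player only if vulnerable and then clearing that vulnerability.
; Each hit tints the player red and launches them away horizontally with slight lift.
; Tick briefly shows the attack flipbook via a delay and calls UpdateAnimation with the idle flipbook for both states.
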(event `self.ReceiveBeginPlay`
  (`KismetSystemLibrary.K2_SetTimerDelegate` (delegate `Melee Attack`) (`self.AttackDelay`) true)
  (set `self.OriginalColor` (`PaperFlipbookComponent.SpriteColor` (`self.Sprite`))))

(event `Melee Attack`
  ;[1 1 1] Atakos logika
  (if (`self.bIsAttacking`)
    (`|ExecutionSequence`
      (:`then_0`
        (set `self.IsAttackAnim` true))
      (:`then_1`
        (bind _as2dside_scroller_character (cast `/Game/2DSideScrollerBP/Blueprints/2DSideScrollerCharacter` (`self.target`)))
        (if (`/Game/2DSideScrollerBP/Blueprints/2DSideScrollerCharacter.IsVulnerable` _as2dside_scroller_character)
          (`|ExecutionSequence`
            (:`then_0`
              (set `/Game/2DSideScrollerBP/Blueprints/2DSideScrollerCharacter.IsVulnerable` false _as2dside_scroller_character))
            (:`then_1`
              (`self.Handle Visuals` _as2dside_scroller_character))
            (:`then_2`
              (`MainCharacter.TakeDamage` _as2dside_scroller_character (`self.BaseDamage`)))))))))

(event `self.ReceiveTick`
  (params (DeltaSeconds :type "Float (single-precision)"))
  ;[1 1 1] Tickas
  (if (`self.IsAttackAnim`)
    (`PaperFlipbookComponent.SetFlipbook` (`self.Sprite`) "/Game/Enemies/MeleeFlyingEnemy/Animations/Attack/Bat_Attack_FB.Bat_Attack_FB")
    (`KismetSystemLibrary.Delay` 0.27)
    (set `self.IsAttackAnim` false))
  (`self.Update Animation` "/Game/Enemies/MeleeFlyingEnemy/Animations/Idle/Bat_Idle_FB.Bat_Idle_FB" "/Game/Enemies/MeleeFlyingEnemy/Animations/Idle/Bat_Idle_FB.Bat_Idle_FB"))

(event `Handle Visuals`
  (params (Player :type "/Game/2DSideScrollerBP/Blueprints/2DSideScrollerCharacter Object Reference"))
  ;[1 1 1] Handles Visuals of taking damage
  (`PaperFlipbookComponent.SetSpriteColor` (`PaperCharacter.Sprite` Player) (struct :`R` 0.642361 :`A` 1.0))
  (if (< (.x (`self.K2_GetActorLocation` Player)) (.x (`self.K2_GetActorLocation`)))
    (`self.LaunchCharacter` Player (-1000.0 0.0 150.0) false false)
    (else
      (`self.LaunchCharacter` Player (1000.0 0.0 150.0) false false))))

(fn `UserConstructionScript`
  (`parent.UserConstructionScript`))