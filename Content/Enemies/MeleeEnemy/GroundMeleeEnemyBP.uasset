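; Ground melee enemy for a 2D side-scroller that patrols, chases players it sees and attacks at close range.
; Tick drives patrol, pursuit of the stored target and flipbook animation, while FrontSight also triggers movement toward seen pawns.
; Overlapping a player capsule with MeleeAttackRange sets the target and starts a looping attack timer, which end overlap clears.
; Each attack plays the swing and, against a vulnerable target, removes vulnerability, tints it red, knocks it away and applies damage.
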(event `self.ReceiveTick`
  (params (DeltaSeconds :type "Float (single-precision)"))
  (bind _target (`self.Target`))
  ;[1 1 1] Tickas
  (`self.Stop Following`)
  (`self.Patrol`)
  (if (`self.IsAttackAnim`)
    (`PaperFlipbookComponent.SetFlipbook` (`self.Sprite`) "/Game/Enemies/MeleeEnemy/Animations/Attack/Melee_Attack_FB.Melee_Attack_FB")
    (`KismetSystemLibrary.Delay` 0.27)
    (set `self.IsAttackAnim` false))
  (`self.UpdateAnimation` "/Game/Enemies/MeleeEnemy/Animations/Idle/Melee_Idle_FB.Melee_Idle_FB" "/Game/Enemies/MeleeEnemy/Animations/Run/Melee_Run_FB.Melee_Run_FB")
  (`/Engine/EditorBlueprintResources/StandardMacros.IsValid` _target
    (:`Is Valid`
      (`self.Move Towards Player` _target))))

(event `self.Front Sight.OnSeePawn`
  (params (Pawn :type "Pawn Object Reference"))
  ;[1 1 1] Kai Pamato zaideja
  (`self.Move Towards Player` Pawn "/Game/Enemies/MeleeEnemy/Animations/Run/Melee_Run_FB.Melee_Run_FB"))

(event `self.Melee Attack Range.OnComponentBeginOverlap`
  (params (OverlappedComponent :type "PrimitiveComponent Object Reference") (OtherActor :type "Actor Object Reference") (OtherComp :type "PrimitiveComponent Object Reference") (OtherBodyIndex :type Integer) (bFromSweep :type Boolean) (SweepResult :type "HitResult Structure (by ref)"))
  (`self.Begin Melee Attack` OtherActor OtherComp (delegate `Melee Attack`)))

(event `self.Melee Attack Range.OnComponentEndOverlap`
  (params (OverlappedComponent :type "PrimitiveComponent Object Reference") (OtherActor :type "Actor Object Reference") (OtherComp :type "PrimitiveComponent Object Reference") (OtherBodyIndex :type Integer))
  (`self.End Melee Attack` OtherActor (delegate `Melee Attack`) OtherComp))

(event `Melee Attack`
  (bind _target (`self.Target`))
  ;[1 1 1] Attack logic
  (`|ExecutionSequence`
    (:`then_0`
      (set `self.IsAttackAnim` true))
    (:`then_1`
      (`/Engine/EditorBlueprintResources/StandardMacros.IsValid` (`self.Target`)
        (:`Is Valid`
          (if (`/Game/2DSideScrollerBP/Blueprints/2DSideScrollerCharacter.IsVulnerable` (`self.Target`))
            (`|ExecutionSequence`
              (:`then_0`
                (set `/Game/2DSideScrollerBP/Blueprints/2DSideScrollerCharacter.IsVulnerable` false _target))
              (:`then_1`
                (`self.Handle Visuals` _target))
              (:`then_2`
                (`MainCharacter.TakeDamage` _target (`self.Base Damage`))))))))))

(event `Handle Visuals`
  (params (Player :type "/Game/2DSideScrollerBP/Blueprints/2DSideScrollerCharacter Object Reference"))
  ;[1 1 1] Handles the visuals of taking damage
  (`PaperFlipbookComponent.SetSpriteColor` (`PaperCharacter.Sprite` Player) (struct :`R` 0.642361 :`A` 1.0))
  (if (< (.x (`self.K2_GetActorLocation` Player)) (.x (`self.K2_GetActorLocation`)))
    (`self.LaunchCharacter` Player (-1000.0 0.0 150.0) false false)
    (else
      (`self.LaunchCharacter` Player (1000.0 0.0 150.0) false false))))

(fn `Begin Melee Attack`
  (params (Object :type "Object Object Reference") (Komponentas :type "ActorComponent Object Reference") (Delegate :type Delegate))
  (bind _as2dside_scroller_character (cast `/Game/2DSideScrollerBP/Blueprints/2DSideScrollerCharacter` Object))
  (cast `CapsuleComponent` Komponentas)
  (set `self.Target` _as2dside_scroller_character)
  (set `self.ShouldAttack` true)
  (`KismetSystemLibrary.K2_SetTimerDelegate` Delegate (`self.AttackDelay`) true)
  (`NavMovementComponent.StopActiveMovement` (`self.CharacterMovement`)))

(fn `End Melee Attack`
  (params (Object :type "Object Object Reference") (Delegate :type Delegate) (Komponentas :type "ActorComponent Object Reference"))
  (cast `/Game/2DSideScrollerBP/Blueprints/2DSideScrollerCharacter` Object)
  (cast `CapsuleComponent` Komponentas)
  (set `self.ShouldAttack` false)
  (`KismetSystemLibrary.K2_SetTimerDelegate` Delegate))

(fn `UserConstructionScript`
  (`parent.UserConstructionScript`))