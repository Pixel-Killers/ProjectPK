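; Flying enemy Blueprint with a flipbook sprite that periodically fires rockets at a target.
; A looping timer, while IsAttacking is set, flags the attack animation and spawns a RocketBP at BulletSpawn aimed at the Target's current location.
; Tick briefly shows the fire flipbook, then returns to idle, which also serves as the move animation.
; DamageNotify briefly tints the sprite red before restoring its original color.
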(event `self.ReceiveBeginPlay`
  (`KismetSystemLibrary.K2_SetTimerDelegate` (delegate `AttackBP`) 2.0 true)
  (set `self.OriginalColor` (`PaperFlipbookComponent.SpriteColor` (`self.Sprite`))))

(event `AttackBP`
  (bind _location (.location (`SceneComponent.K2_GetComponentToWorld` (`self.BulletSpawn`))))
  ;[1 1 1] Atakos logika
  (if (`self.bIsAttacking`)
    (`|ExecutionSequence`
      (:`then_0`
        (set `self.IsAttackAnim` true))
      (:`then_1`
        (bind _returnvalue (`|SpawnActorFromClass` "/Game/Enemies/RangedAttack/Animations/Rocket/RocketBP.RocketBP_C" (`KismetMathLibrary.MakeTransform` _location (`KismetMathLibrary.FindLookAtRotation` _location (`self.K2_GetActorLocation` (`self.target`))) (.scale (`SceneComponent.K2_GetComponentToWorld` (`self.BulletSpawn`)))) "Undefined" "OverrideRootScale" null null))
        (set `/Game/Enemies/RangedAttack/Animations/RangedAttack.BaseDamage` 20 _returnvalue)))))

(event `self.ReceiveTick`
  (params (DeltaSeconds :type "Float (single-precision)"))
  ;[1 1 1] Tick'as
  (if (`self.IsAttackAnim`)
    (`PaperFlipbookComponent.SetFlipbook` (`self.Sprite`) "/Game/Enemies/FlyingEnemy/Animations/Fire/FlyingEnemy_Fire.FlyingEnemy_Fire")
    (`KismetSystemLibrary.Delay` 0.27)
    (set `self.IsAttackAnim` false))
  (`self.Update Animation` "/Game/Enemies/FlyingEnemy/Animations/Idle/FlyingEnemy_Idle.FlyingEnemy_Idle" "/Game/Enemies/FlyingEnemy/Animations/Idle/FlyingEnemy_Idle.FlyingEnemy_Idle"))

(event `DamageNotify`
  ;[1 1 1] Parodo, kad patyre zala
  (`PaperFlipbookComponent.SetSpriteColor` (`self.Sprite`) (struct :`R` 0.642361 :`A` 1.0))
  (`KismetSystemLibrary.Delay` 0.3)
  (`PaperFlipbookComponent.SetSpriteColor` (`self.Sprite`) (`self.OriginalColor`)))

(fn `Update Animation`
  (params (Idle :type "PaperFlipbook Object Reference") (Move :type "PaperFlipbook Object Reference"))
  (`PaperFlipbookComponent.SetFlipbook` (`self.Sprite`) (select `bool` (> (`KismetMathLibrary.VSize` (`self.GetVelocity`)) 0.0) :`false` Idle :`true` Move))
  (return))

(fn `UserConstructionScript`)