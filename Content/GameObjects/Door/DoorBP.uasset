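; A 2D door Blueprint that the player opens and closes with the F key while near it.
; Overlap events on a Box component enable and disable the first player controller's input on the door, without filtering the overlapping actor.
; F toggles the Open flag and the PaperSprite's collision, with inverted naming: Open true means solid.
; Printed strings stand in for animations.
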(event `Key|F`
  (params (Key :type "Key Structure"))
  (bind _papersprite (`self.PaperSprite`))
  ;[1 1 1] Open/Close Door
  (:`Pressed`
    (if (`self.Open`)
      (set `self.Open` false)
      (`PrimitiveComponent.SetCollisionEnabled` _papersprite "NoCollision")
      (`KismetSystemLibrary.PrintString` "open anim")
      (else
        (set `self.Open` true)
        (`PrimitiveComponent.SetCollisionEnabled` _papersprite "QueryAndPhysics")
        (`KismetSystemLibrary.PrintString` "closed anim")))))

(event `self.Box.OnComponentBeginOverlap`
  (params (OverlappedComponent :type "PrimitiveComponent Object Reference") (OtherActor :type "Actor Object Reference") (OtherComp :type "PrimitiveComponent Object Reference") (OtherBodyIndex :type Integer) (bFromSweep :type Boolean) (SweepResult :type "HitResult Structure (by ref)"))
  ;[1 1 1] Enable Inputs
  (`self.EnableInput` (`GameplayStatics.GetPlayerController` 0)))

(event `self.Box.OnComponentEndOverlap`
  (params (OverlappedComponent :type "PrimitiveComponent Object Reference") (OtherActor :type "Actor Object Reference") (OtherComp :type "PrimitiveComponent Object Reference") (OtherBodyIndex :type Integer))
  ;[1 1 1] Enable Inputs
  (`self.DisableInput` (`GameplayStatics.GetPlayerController` 0)))

(fn `UserConstructionScript`)